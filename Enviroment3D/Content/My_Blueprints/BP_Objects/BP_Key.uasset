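; BP_Key is a key pickup that shows an interaction prompt when the player is near.
; It creates a WB_TakeKey widget at BeginPlay, then adds it to or removes it from the viewport as the player character enters or leaves its box collision.
; The Interact event calls PickUPKeyMessage on the referenced Door and destroys the key actor.
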(event `/Game/My_Blueprints/BP_Objects/BPI_KeyDoor.Interact`
  (message `/Game/My_Blueprints/BP_Objects/BPI_DoorSystem.PickUPKey` (`self.Door`))
  (`self.K2_DestroyActor`))

(event `self.ReceiveBeginPlay`
  (bind _returnvalue (`|CreateWidget` "/Game/Interfaces/WB_TakeKey.WB_TakeKey_C"))
  (set `self.InteractPromptKeyWB` _returnvalue))

(event `self.BoxCollisionKeyInterface.OnComponentBeginOverlap`
  (params (OverlappedComponent :type "PrimitiveComponent Object Reference") (OtherActor :type "Actor Object Reference") (OtherComp :type "PrimitiveComponent Object Reference") (OtherBodyIndex :type Integer) (bFromSweep :type Boolean) (SweepResult :type "HitResult Structure (by ref)"))
  (if (== OtherActor (`GameplayStatics.GetPlayerCharacter` 0))
    (`UserWidget.AddToViewport` (`self.InteractPromptKeyWB`) 0)))

(event `self.BoxCollisionKeyInterface.OnComponentEndOverlap`
  (params (OverlappedComponent :type "PrimitiveComponent Object Reference") (OtherActor :type "Actor Object Reference") (OtherComp :type "PrimitiveComponent Object Reference") (OtherBodyIndex :type Integer))
  (if (== (`GameplayStatics.GetPlayerCharacter` 0) OtherActor)
    (`Widget.RemoveFromParent` (`self.InteractPromptKeyWB`))))

(fn `UserConstructionScript`)