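; BP_Dissolve1 is a proximity trigger that shows an on-screen interaction prompt when the player is near.
; It creates the WB_Disolve1 widget once at BeginPlay and keeps it for reuse.
; Its SphereCollision overlap events add the widget to the viewport when player character 0 enters and remove it on exit.
; No dissolve logic exists in its graphs.
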(event `self.ReceiveBeginPlay`
  (bind _returnvalue (`|CreateWidget` "/Game/Interfaces/WB_Disolve1.WB_Disolve1_C"))
  (set `self.WB_interactivePrompt` _returnvalue))

(event `self.sphereCollision.OnComponentBeginOverlap`
  (params (OverlappedComponent :type "PrimitiveComponent Object Reference") (OtherActor :type "Actor Object Reference") (OtherComp :type "PrimitiveComponent Object Reference") (OtherBodyIndex :type Integer) (bFromSweep :type Boolean) (SweepResult :type "HitResult Structure (by ref)"))
  (if (== OtherActor (`GameplayStatics.GetPlayerCharacter` 0))
    (`UserWidget.AddToViewport` (`self.WB_interactivePrompt`) 0)))

(event `self.sphereCollision.OnComponentEndOverlap`
  (params (OverlappedComponent :type "PrimitiveComponent Object Reference") (OtherActor :type "Actor Object Reference") (OtherComp :type "PrimitiveComponent Object Reference") (OtherBodyIndex :type Integer))
  (if (== (`GameplayStatics.GetPlayerCharacter` 0) OtherActor)
    (`Widget.RemoveFromParent` (`self.WB_interactivePrompt`))))

(fn `UserConstructionScript`)