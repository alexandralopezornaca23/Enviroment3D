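; BP_Door is a key-locked door that opens on Interact once PickUPKey has set its Llave flag.
; A FlipFlop plays a timeline that lerps the root's roll to open it; only the A output is wired, so there is no closing action.
; A collision box shows the WB_OpenDoor prompt to the player and destroys itself shortly after they leave, making the prompt one-time.
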(event `/Game/My_Blueprints/BP_Objects/BPI_KeyDoor.Interact`
  (if (`self.Llave`)
    (`/Engine/EditorBlueprintResources/StandardMacros.FlipFlop`
      (:`A`
        (bind (_direction _doortrack) (`Timeline|Door TimeLine`)
          (:`Update`
            (`SceneComponent.K2_SetRelativeRotation` (`self.DefaultSceneRoot`) (`KismetMathLibrary.MakeRotator` (`KismetMathLibrary.Lerp` 0.0 -90.0 _doortrack)) false false)))))))

(event `/Game/My_Blueprints/BP_Objects/BPI_DoorSystem.PickUPKey`
  (set `self.Llave` true))

(event `self.ReceiveBeginPlay`
  (bind _returnvalue (`|CreateWidget` "/Game/Interfaces/WB_OpenDoor.WB_OpenDoor_C"))
  (set `self.InteractPromptWB` _returnvalue))

(event `self.BoxCollisionWPDoor.OnComponentBeginOverlap`
  (params (OverlappedComponent :type "PrimitiveComponent Object Reference") (OtherActor :type "Actor Object Reference") (OtherComp :type "PrimitiveComponent Object Reference") (OtherBodyIndex :type Integer) (bFromSweep :type Boolean) (SweepResult :type "HitResult Structure (by ref)"))
  (if (== OtherActor (`GameplayStatics.GetPlayerCharacter` 0))
    (`UserWidget.AddToViewport` (`self.InteractPromptWB`) 0)))

(event `self.BoxCollisionWPDoor.OnComponentEndOverlap`
  (params (OverlappedComponent :type "PrimitiveComponent Object Reference") (OtherActor :type "Actor Object Reference") (OtherComp :type "PrimitiveComponent Object Reference") (OtherBodyIndex :type Integer))
  (if (== (`GameplayStatics.GetPlayerCharacter` 0) OtherActor)
    (`Widget.RemoveFromParent` (`self.InteractPromptWB`))
    (`KismetSystemLibrary.Delay` 0.05)
    (`ActorComponent.K2_DestroyComponent` (`self.BoxCollisionWPDoor`))))

(fn `UserConstructionScript`)