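; BP_Octavia is a playable character Blueprint with third-person-style movement, look, jump and a melee attack.
; BeginPlay adds the Enhanced Input movement context and clamps camera pitch to a narrow range.
; Attacking, allowed only while walking, disables movement and plays a montage whose notifies toggle the hitbox collision and restore walking.
; Actors that begin overlapping the attack box receive fixed damage.
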(event `self.ReceiveBeginPlay`
  (bind _returnvalue (`GameplayStatics.GetPlayerCameraManager` 0))
  (bind _returnvalue_2 (pcsubsystem `EnhancedInputLocalPlayerSubsystem` (`GameplayStatics.GetPlayerController` 0)))
  (`|ExecutionSequence`
    (:`then_0`
      ;[1 0.5059 0.7916] Input behavior
      (`/Engine/EditorBlueprintResources/StandardMacros.IsValid` _returnvalue_2
        (:`Is Valid`
          (`EnhancedInputSubsystemInterface.AddMappingContext` _returnvalue_2 "/Game/Octavia_Character/IMC_Movement.IMC_Movement" 0 (struct)))))
    (:`then_1`
      (set `PlayerCameraManager.ViewPitchMin` 10.0 _returnvalue)
      (set `PlayerCameraManager.ViewPitchMax` 20.0 _returnvalue))))

(event `EnhancedInput|/Game/Octavia_Character/INP_Jump`
  (params (ActionValue :type Boolean) (ElapsedSeconds :type "Float (double-precision)") (TriggeredSeconds :type "Float (double-precision)") (InputAction :type "InputAction Object Reference" :default "/Game/Octavia_Character/INP_Jump.INP_Jump"))
  ;[1 1 1] Input Jump
  (:`Started`
    (`self.Jump`))
  (:`Completed`
    (`self.StopJumping`)))

(event `EnhancedInput|/Game/Octavia_Character/INP_LookArround`
  (params (ActionValue :type "Vector2D Structure") (ElapsedSeconds :type "Float (double-precision)") (TriggeredSeconds :type "Float (double-precision)") (InputAction :type "InputAction Object Reference" :default "/Game/Octavia_Character/INP_LookArround.INP_LookArround"))
  ;[1 1 1] Input Look Arround
  (:`Triggered`
    (`self.AddControllerYawInput` ActionValue_X)
    (`self.AddControllerPitchInput` ActionValue_Y)))

(event `EnhancedInput|/Game/Octavia_Character/INP_MoveArround`
  (params (ActionValue :type "Vector2D Structure") (ElapsedSeconds :type "Float (double-precision)") (TriggeredSeconds :type "Float (double-precision)") (InputAction :type "InputAction Object Reference" :default "/Game/Octavia_Character/INP_MoveArround.INP_MoveArround"))
  (bind (_returnvalue_roll _returnvalue_pitch _returnvalue_yaw) (`KismetMathLibrary.BreakRotator` (`self.GetControlRotation`)))
  ;[1 1 1] Input Movement
  (:`Triggered`
    (`self.AddMovementInput` (`KismetMathLibrary.GetRightVector` (`self.GetControlRotation`)) ActionValue_X)
    (`self.AddMovementInput` (`KismetMathLibrary.GetForwardVector` (`KismetMathLibrary.MakeRotator` _returnvalue_roll 0.0 _returnvalue_yaw)) ActionValue_Y)))

(event `EnhancedInput|/Game/Octavia_Character/INP_Attack`
  (params (ActionValue :type Boolean) (ElapsedSeconds :type "Float (double-precision)") (TriggeredSeconds :type "Float (double-precision)") (InputAction :type "InputAction Object Reference" :default "/Game/Octavia_Character/INP_Attack.INP_Attack"))
  (:`Started`
    (switch `EMovementMode` (`CharacterMovementComponent.MovementMode` (`self.CharacterMovement`))
      (:`MOVE_Walking`
        (`CharacterMovementComponent.SetMovementMode` (`self.CharacterMovement`) "MOVE_None" 0)
        (bind _notifyname (`|PlayMontage` (`self.Mesh`) "/Game/Octavia_Character/Animation_Character/Anim_Montages/AM_Attack004.AM_Attack004")
          (:`OnNotifyBegin`
            (switch `name` _notifyname
              (:`AttackStart`
                (`PrimitiveComponent.SetCollisionProfileName` (`self.Attack_BoxCollision`) "OverlapAllDynamic" true))
              (:`AttackEnd`
                (`PrimitiveComponent.SetCollisionProfileName` (`self.Attack_BoxCollision`) "NoCollision" true))
              (:`AnimStop`
                (`CharacterMovementComponent.SetMovementMode` (`self.CharacterMovement`) "MOVE_Walking" 0)))))))))

(event `self.Attack_BoxCollision.OnComponentBeginOverlap`
  (params (OverlappedComponent :type "PrimitiveComponent Object Reference") (OtherActor :type "Actor Object Reference") (OtherComp :type "PrimitiveComponent Object Reference") (OtherBodyIndex :type Integer) (bFromSweep :type Boolean) (SweepResult :type "HitResult Structure (by ref)"))
  (`GameplayStatics.ApplyDamage` OtherActor 10.0 null self))

(fn `UserConstructionScript`)