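; BP_Trigger2 is a placed trigger that lets Octavia start a drink-potion cinematic and shows its interaction prompt.
; Entering the Box registers the trigger on BP_Octavia as BPTrigger02 and sets the Dentro flag, which clears on exit.
; PlayCinematics, not called within this Blueprint, plays the LS_Character_002 level sequence.
; A separate Trigger_Interfaz_002 volume adds and removes the WB_DrinkPotion widget, created at BeginPlay, for the player character.
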(event `self.Box.OnComponentBeginOverlap`
  (params (OverlappedComponent :type "PrimitiveComponent Object Reference") (OtherActor :type "Actor Object Reference") (OtherComp :type "PrimitiveComponent Object Reference") (OtherBodyIndex :type Integer) (bFromSweep :type Boolean) (SweepResult :type "HitResult Structure (by ref)"))
  (bind _asbp_octavia (cast `/Game/Octavia_Character/BP_Octavia` OtherActor))
  (set `/Game/Octavia_Character/BP_Octavia.BP_Trigger02` self _asbp_octavia)
  (set `self.Dentro` true))

(event `self.Box.OnComponentEndOverlap`
  (params (OverlappedComponent :type "PrimitiveComponent Object Reference") (OtherActor :type "Actor Object Reference") (OtherComp :type "PrimitiveComponent Object Reference") (OtherBodyIndex :type Integer))
  (cast `/Game/Octavia_Character/BP_Octavia` OtherActor)
  (set `self.Dentro` false))

(event `PlayCinematics`
  (`LevelSequencePlayer.CreateLevelSequencePlayer` "/Game/Cinematicas/LS_Character_002.LS_Character_002")
  (`MovieSceneSequencePlayer.Play` (`LevelSequenceActor.SequencePlayer` (`self.Sequence Player`))))

(event `self.ReceiveBeginPlay`
  (bind _returnvalue (`|CreateWidget` "/Game/Interfaces/WB_DrinkPotion.WB_DrinkPotion_C"))
  (set `self.InteractionPrompt` _returnvalue))

(event `self.Trigger_Interfaz_002.OnComponentBeginOverlap`
  (params (OverlappedComponent :type "PrimitiveComponent Object Reference") (OtherActor :type "Actor Object Reference") (OtherComp :type "PrimitiveComponent Object Reference") (OtherBodyIndex :type Integer) (bFromSweep :type Boolean) (SweepResult :type "HitResult Structure (by ref)"))
  (if (== OtherActor (`GameplayStatics.GetPlayerCharacter` 0))
    (`UserWidget.AddToViewport` (`self.InteractionPrompt`) 0)))

(event `self.Trigger_Interfaz_002.OnComponentEndOverlap`
  (params (OverlappedComponent :type "PrimitiveComponent Object Reference") (OtherActor :type "Actor Object Reference") (OtherComp :type "PrimitiveComponent Object Reference") (OtherBodyIndex :type Integer))
  (if (== (`GameplayStatics.GetPlayerCharacter` 0) OtherActor)
    (`Widget.RemoveFromParent` (`self.InteractionPrompt`))))

(fn `UserConstructionScript`)